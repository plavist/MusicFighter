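; YBOT_BP is an AI pawn that takes sword damage and pins the player when close.
; Overlap with BP_Weapon_Sword subtracts the sword's damage from Health, destroying the pawn at zero, gated by CanDamage copied each tick from ThirdPersonCharacter.
; Tick also clears the player's CanMove within close range and spawns a Widget actor once, offset randomly from the pawn.
; A random navmesh wander using AIMoveTo exists but is never triggered.
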(event EventTick
  (params (DeltaSeconds :type Float%20%28single-precision%29))
  (Utilities|FlowControl|Sequence
    (:then_0
      (bind _asthird_person_character (Utilities|Casting|CastToThirdPersonCharacter (Game|GetPlayerCharacter 0)))
      (Variables|Default|SetCan%20Damage (Variables|/Game/ThirdPersonBP/Blueprints/ThirdPersonCharacter.ThirdPersonCharacter_C|GetCanDamage _asthird_person_character)))
    (:then_1
      (if (< (Math|Vector|VectorLength (- (Transformation|GetActorLocation (Game|GetPlayerCharacter 0)) (Transformation|GetActorLocation))) 1.5e+02)
        (Variables|/Game/ThirdPersonBP/Blueprints/ThirdPersonCharacter.ThirdPersonCharacter_C|SetCanMove _asthird_person_character false)
        (if (not (Variables|Default|GetisWidget))
          (Game|SpawnActorfromClass "/Game/Widget.Widget_C" (Math|Conversions|ToTransform(Vector) (Math|Transform|TransformLocation (Transformation|GetActorTransform) (Math|Vector|MakeVector 2e+01 (Math|Random|RandomFloatinRange 0.0 4e+01) (Math|Random|RandomFloatinRange 0.0 4e+01)))) "Undefined" 0 0)
          (Variables|Default|SetisWidget true))))))

(event Collision|EventActorBeginOverlap
  (params (OtherActor :type Actor%20Object%20Reference))
  (if (Variables|Default|GetCan%20Damage)
    (bind _asbp_weapon_sword (Utilities|Casting|CastToBP_Weapon_Sword OtherActor))
    (Development|PrintString "ya" true true "(R=0.000000,G=0.660000,B=1.000000,A=1.000000)" 0.0)
    (Variables|Default|SetHealth (- (Variables|Default|GetHealth) (Variables|/Game/ThirdPersonBP/Blueprints/BP_Weapon_Master.BP_Weapon_Master_C|GetDamage _asbp_weapon_sword)))
    (if (<= (Variables|Default|GetHealth) 0.0)
      (Actor|DestroyActor))))

(fn ConstructionScript)