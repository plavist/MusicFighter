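; YBOT_BP is a YBot character that takes damage and dies as a ragdoll.
; Any damage lowers Health and prints it, and Tick calls DEATH whenever Health is zero or below.
; DEATH sets IsDead, briefly waits, disables capsule collision, enables mesh physics, then destroys the actor after a longer delay.
; Random navmesh wandering and a player-proximity Widget spawn are present but disconnected, so neither runs.
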(event Custom|DEATH
  (Variables|Default|SetisDead true)
  (Utilities|FlowControl|Delay 0.4)
  (Collision|SetCollisionEnabled (Variables|Collision|GetCapsuleComponent) "NoCollision")
  (Physics|SetSimulatePhysics (Variables|Character|GetMesh) true)
  (Collision|SetCollisionEnabled (Variables|Character|GetMesh) "QueryAndPhysics")
  (Utilities|FlowControl|Delay 15.0)
  (Actor|DestroyActor))

(event EventTick
  (params (DeltaSeconds :type Float%20%28single-precision%29))
  (if (<= (Variables|Default|GetHealth) 0.0)
    (CallFunction|DEATH)))

(event Game|Damage|EventAnyDamage
  (params (Damage :type Float%20%28single-precision%29) (DamageType :type Damage%20Type%20Object%20Reference) (InstigatedBy :type Controller%20Object%20Reference) (DamageCauser :type Actor%20Object%20Reference))
  (bind _output_get (Variables|Default|SetHealth (- (Variables|Default|GetHealth) Damage)))
  (Development|PrintString (Utilities|String|ToString(Float) _output_get) true true "(R=0.000000,G=0.660000,B=1.000000,A=1.000000)" 1e+04))

(fn ConstructionScript)